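; BP_Mine is a proximity mine that the third-person character arms by touching it, with debug prints standing in for explosion and damage.
; MineCollision overlap fires once, swapping the mesh material and running a timeline that animates its Switch parameter and enables DamageZone queries.
; Character overlap with DamageZone starts a short fuse, then prints a hit or escape depending on whether the player is still inside, destroying the mine either way.
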(event `self.ReceiveBeginPlay`
  (`PrimitiveComponent.SetCollisionEnabled` (`self.DamageZone`) "NoCollision"))

(event `self.MineCollision.OnComponentBeginOverlap`
  (params (OverlappedComponent :type "PrimitiveComponent Object Reference") (OtherActor :type "Actor Object Reference") (OtherComp :type "PrimitiveComponent Object Reference") (OtherBodyIndex :type Integer) (bFromSweep :type Boolean) (SweepResult :type "HitResult Structure (by ref)"))
  (bind _minemesh (`self.MineMesh`))
  (cast `/Game/CosmicPlatformer/Blueprints/Player/ThirdPersonCharacter` OtherActor)
  (`/Engine/EditorBlueprintResources/StandardMacros.DoOnce` false
    (:`Completed`
      (`KismetSystemLibrary.PrintString` "TicTac")
      (`PrimitiveComponent.SetMaterial` _minemesh 0 "/Game/CosmicPlatformer/Blueprints/Sandbox/Mines/MI_Mine.MI_Mine")
      (bind (_direction _newtrack_0) (`Timeline|MineTL` :!via `PlayFromStart`)
        (:`Update`
          (`MeshComponent.SetScalarParameterValueOnMaterials` _minemesh "Switch" _newtrack_0)
          (`PrimitiveComponent.SetCollisionEnabled` (`self.DamageZone`) "QueryOnly"))))))

(event `self.DamageZone.OnComponentBeginOverlap`
  (params (OverlappedComponent :type "PrimitiveComponent Object Reference") (OtherActor :type "Actor Object Reference") (OtherComp :type "PrimitiveComponent Object Reference") (OtherBodyIndex :type Integer) (bFromSweep :type Boolean) (SweepResult :type "HitResult Structure (by ref)"))
  (cast `/Game/CosmicPlatformer/Blueprints/Player/ThirdPersonCharacter` OtherActor)
  (`KismetSystemLibrary.Delay` 1.5)
  (`KismetSystemLibrary.PrintString` "Boom")
  (if (`PrimitiveComponent.IsOverlappingActor` (`self.DamageZone`) (`GameplayStatics.GetPlayerCharacter` 0))
    (`KismetSystemLibrary.PrintString` "Aie")
    (`self.K2_DestroyActor`)
    (else
      (`KismetSystemLibrary.PrintString` "Ouf")
      (`self.K2_DestroyActor`))))

(fn `UserConstructionScript`)
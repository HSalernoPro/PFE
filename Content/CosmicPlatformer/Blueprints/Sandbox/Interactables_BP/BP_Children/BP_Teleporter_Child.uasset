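; Two-way teleporter interactable, a child Blueprint that moves the player character between a start point and an arrival point on interaction.
; Overlaps on Box and BoxArrival set IsAtStart to track which end the player is at, and BoxArrival also sets or clears the character's interactable reference.
; InteractionStart uses that flag to place the player at the opposite cube's world location.
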(event `self.Interaction_Start`
  (bind _asthird_person_character (cast `/Game/CosmicPlatformer/Blueprints/Player/ThirdPersonCharacter` (`GameplayStatics.GetPlayerCharacter` 0) :!pure true))
  (if (`self.IsAtStart?`)
    (`self.K2_SetActorLocation` _asthird_person_character (`SceneComponent.K2_GetComponentLocation` (`self.CubeArrival`)) false false)
    (else
      (`self.K2_SetActorLocation` _asthird_person_character (`SceneComponent.K2_GetComponentLocation` (`self.CubeStart`)) false false))))

(event `self.BoxArrival.OnComponentBeginOverlap`
  (params (OverlappedComponent :type "PrimitiveComponent Object Reference") (OtherActor :type "Actor Object Reference") (OtherComp :type "PrimitiveComponent Object Reference") (OtherBodyIndex :type Integer) (bFromSweep :type Boolean) (SweepResult :type "HitResult Structure (by ref)"))
  (bind _asthird_person_character (cast `/Game/CosmicPlatformer/Blueprints/Player/ThirdPersonCharacter` OtherActor))
  (set `/Game/CosmicPlatformer/Blueprints/Player/ThirdPersonCharacter.Ref_Interactable_Parent` self _asthird_person_character)
  (set `self.IsAtStart?` false))

(event `self.BoxArrival.OnComponentEndOverlap`
  (params (OverlappedComponent :type "PrimitiveComponent Object Reference") (OtherActor :type "Actor Object Reference") (OtherComp :type "PrimitiveComponent Object Reference") (OtherBodyIndex :type Integer))
  (bind _asthird_person_character (cast `/Game/CosmicPlatformer/Blueprints/Player/ThirdPersonCharacter` OtherActor))
  (set `/Game/CosmicPlatformer/Blueprints/Player/ThirdPersonCharacter.Ref_Interactable_Parent` null _asthird_person_character))

(event `self.Box.OnComponentBeginOverlap`
  (params (OverlappedComponent :type "PrimitiveComponent Object Reference") (OtherActor :type "Actor Object Reference") (OtherComp :type "PrimitiveComponent Object Reference") (OtherBodyIndex :type Integer) (bFromSweep :type Boolean) (SweepResult :type "HitResult Structure (by ref)"))
  (cast `/Game/CosmicPlatformer/Blueprints/Player/ThirdPersonCharacter` OtherActor)
  (set `self.IsAtStart?` true))

(event `self.Box.OnComponentEndOverlap`
  (params (OverlappedComponent :type "PrimitiveComponent Object Reference") (OtherActor :type "Actor Object Reference") (OtherComp :type "PrimitiveComponent Object Reference") (OtherBodyIndex :type Integer))
  (cast `/Game/CosmicPlatformer/Blueprints/Player/ThirdPersonCharacter` OtherActor))

(fn `UserConstructionScript`
  (`parent.UserConstructionScript`))
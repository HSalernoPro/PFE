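; Interactable child Blueprint that spawns a moving platform and toggles its movement on interaction.
; On BeginPlay it caches the start and arrival marker locations, destroys both markers and spawns a BP_MovingPlateform at the start.
; It passes its movement and respawn settings to that platform, forces it non-breakable and stops its timeline.
; InteractionStart uses a FlipFlop to alternately start the platform, recalling its speed, and stop it.
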(event `self.ReceiveBeginPlay`
  (bind _plateformstart (`self.PlateformStart`))
  (bind _plateformarrival (`self.PlateformArrival`))
  (set `self.StartLocation` (`SceneComponent.K2_GetComponentLocation` _plateformstart))
  (`ActorComponent.K2_DestroyComponent` _plateformstart)
  (set `self.TargetedLocation` (`SceneComponent.K2_GetComponentLocation` _plateformarrival))
  (`ActorComponent.K2_DestroyComponent` _plateformarrival)
  (bind _returnvalue (`|SpawnActorFromClass` "/Game/CosmicPlatformer/Assets/Actors/Moving_Plateform/BP_MovingPlateform.BP_MovingPlateform_C" (`KismetMathLibrary.MakeTransform` (`self.StartLocation`) (struct) (`self.PlateformScale`)) "Undefined" "OverrideRootScale" null null))
  (bind _output_get (set `self.Ref_MovingPlateform` _returnvalue))
  (set `/Game/CosmicPlatformer/Assets/Actors/Moving_Plateform/BP_MovingPlateform.TargetedLocation` (`self.TargetedLocation`) _output_get)
  (set `/Game/CosmicPlatformer/Assets/Actors/Moving_Plateform/BP_MovingPlateform.MovingPlateform?` true _output_get)
  (set `/Game/CosmicPlatformer/Assets/Actors/Moving_Plateform/BP_MovingPlateform.Loop?` (`self.Loop?`) _output_get)
  (set `/Game/CosmicPlatformer/Assets/Actors/Moving_Plateform/BP_MovingPlateform.TriggerActivation?` false _output_get)
  (set `/Game/CosmicPlatformer/Assets/Actors/Moving_Plateform/BP_MovingPlateform.PlateformSpeed` (`self.PlateformSpeed`) _output_get)
  (set `/Game/CosmicPlatformer/Assets/Actors/Moving_Plateform/BP_MovingPlateform.Breakable?` false _output_get)
  (set `/Game/CosmicPlatformer/Assets/Actors/Moving_Plateform/BP_MovingPlateform.NTimesToBreak` (`self.NTimesToBreak`) _output_get)
  (set `/Game/CosmicPlatformer/Assets/Actors/Moving_Plateform/BP_MovingPlateform.RespawnTime` (`self.RespawnTime`) _output_get)
  (set `/Game/CosmicPlatformer/Assets/Actors/Moving_Plateform/BP_MovingPlateform.ForceRespawnAtStartLocation?` (`self.ForceRespawnAtStartLocation?`) _output_get)
  (set `/Game/CosmicPlatformer/Assets/Actors/Moving_Plateform/BP_MovingPlateform.WasOn?` false _output_get)
  (`TimelineComponent.Stop` (`/Game/CosmicPlatformer/Assets/Actors/Moving_Plateform/BP_MovingPlateform.Movement_Timeline` _output_get)))

(event `self.Interaction_Start`
  (bind _ref_movingplateform (`self.Ref_MovingPlateform`))
  (`/Engine/EditorBlueprintResources/StandardMacros.FlipFlop`
    (:`A`
      (`/Game/CosmicPlatformer/Assets/Actors/Moving_Plateform/BP_MovingPlateform.StartThxToTrigger` _ref_movingplateform)
      (set `/Game/CosmicPlatformer/Assets/Actors/Moving_Plateform/BP_MovingPlateform.WasOn?` true _ref_movingplateform)
      (`/Game/CosmicPlatformer/Assets/Actors/Moving_Plateform/BP_MovingPlateform.RecallSpeed` _ref_movingplateform))
    (:`B`
      (`/Game/CosmicPlatformer/Assets/Actors/Moving_Plateform/BP_MovingPlateform.StopThxToTrigger` _ref_movingplateform)
      (set `/Game/CosmicPlatformer/Assets/Actors/Moving_Plateform/BP_MovingPlateform.WasOn?` true _ref_movingplateform))))

(fn `UserConstructionScript`
  (`parent.UserConstructionScript`))
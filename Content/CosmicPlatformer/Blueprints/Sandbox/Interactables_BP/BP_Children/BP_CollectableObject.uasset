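; BP_CollectableObject is an interactable pickup that can switch in and out of the world with timeline swaps.
; Each SwapTimeline event alternately hides it, disabling collision and physics, or restores all three.
; Interacting while not hidden stores a self reference in the player character's ObjectStored, then destroys the actor.
; Box overlap prints the object's name on screen.
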(event `SwapTimeline`
  (bind _formtoattachboxcoll (`self.FormToAttachBoxColl`))
  (`/Engine/EditorBlueprintResources/StandardMacros.FlipFlop`
    (:`A`
      (`self.SetActorHiddenInGame` true)
      (`self.SetActorEnableCollision` false)
      (`PrimitiveComponent.SetSimulatePhysics` _formtoattachboxcoll false))
    (:`B`
      (`self.SetActorHiddenInGame` false)
      (`self.SetActorEnableCollision` true)
      (`PrimitiveComponent.SetSimulatePhysics` _formtoattachboxcoll true))))

(event `self.Interaction_Start`
  (if (not (`self.bHidden`))
    (bind _asthird_person_character (cast `/Game/CosmicPlatformer/Blueprints/Player/ThirdPersonCharacter` (`GameplayStatics.GetPlayerCharacter` 0)))
    (set `/Game/CosmicPlatformer/Blueprints/Player/ThirdPersonCharacter.ObjectStored` self _asthird_person_character)
    (`self.K2_DestroyActor`)))

(event `self.Box.OnComponentBeginOverlap`
  (params (OverlappedComponent :type "PrimitiveComponent Object Reference") (OtherActor :type "Actor Object Reference") (OtherComp :type "PrimitiveComponent Object Reference") (OtherBodyIndex :type Integer) (bFromSweep :type Boolean) (SweepResult :type "HitResult Structure (by ref)"))
  (`KismetSystemLibrary.PrintString` (`KismetTextLibrary.Conv_TextToString` (`self.NameOfTheObj`)) true true (struct :`R` 1.0 :`A` 1.0) 3.0))

(fn `UserConstructionScript`
  (`parent.UserConstructionScript`))
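; BP_PNJ is an interactable NPC that shows dialogue on interaction, as either a Major or Minor character.
; A Major NPC absorbs the player's Major Fragments up to the number it lacks, then shows the dialogue line indexed by its fragment count.
; A Minor NPC shows a single fixed line.
; Both write text through a typewriter-style WB_Text_to_write widget, whose finished event clears the dialogue after a short delay.
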(event `self.Interaction_Start`
  ;[1 1 1] Check what type of NPC it is? (Major or Minor)
  (bind _output_get (set `self.NPC_Matters_Enum` (`self.NPC_Matters_Enum`)))
  (switch `/Game/CosmicPlatformer/Blueprints/Sandbox/Interactables_BP/BP_Children/NPC_Matters` _output_get
    (:`NewEnumerator0`
      ;[1 1 1] If Major, sets the Array to the number of Fragments needed for full speech
      (set `self.NbFragmentsNeeded` (- (`KismetArrayLibrary.Array_Length` (`self.MajorNPC_Dialogues`)) 1))
      ;[1 1 1] Check if NPC is already having all its Fragments, if True, immediately display the text
      (bind _asthird_person_character (cast `/Game/CosmicPlatformer/Blueprints/Player/ThirdPersonCharacter` (`GameplayStatics.GetPlayerCharacter` 0)))
      (set `self.Ref_TPC` _asthird_person_character)
      (if (== (`self.NbFragmentsNeeded`) (`self.CurrentNbFragments`))
        ;[1 1 1] Display text depending on the current number of Fragments
        (set `self.TexteToFill` (`|GetArrayItem` (`self.MajorNPC_Dialogues`) (`self.CurrentNbFragments`)) :!label _label)
        (bind _returnvalue (`|CreateWidget` "/Game/CosmicPlatformer/Blueprints/Sandbox/Interactables_BP/BP_Children/WB_Text_to_write.WB_Text_to_write_C" (`GameplayStatics.GetPlayerController` 0) (`self.CharactersPerSeconds`) :!label _label_2))
        (`WidgetComponent.SetWidget` (`self.Widget_Dialogue`) _returnvalue)
        (add `/Game/CosmicPlatformer/Blueprints/Sandbox/Interactables_BP/BP_Children/WB_Text_to_write.FinishedWriting` _returnvalue (delegate `Disappear`))
        (`/Game/CosmicPlatformer/Blueprints/Sandbox/Interactables_BP/BP_Children/WB_Text_to_write.Write` _returnvalue (`self.TexteToFill`))
        (else
          ;[1 1 1] If not, check how many are missing
          (set `self.NbFragmentsMissing` (- (`self.NbFragmentsNeeded`) (`self.CurrentNbFragments`)))
          ;[1 1 1] Check if the TPC has less or the exact number of Fragments needed
          (if (<= (`/Game/CosmicPlatformer/Blueprints/Player/ThirdPersonCharacter.MajorFragment` (`self.Ref_TPC`)) (`self.NbFragmentsMissing`))
            ;[1 1 1] If True, gives all its Fragments to the NPC, and sets TPC's number of Fragments to 0
            (set `self.CurrentNbFragments` (+ (`/Game/CosmicPlatformer/Blueprints/Player/ThirdPersonCharacter.MajorFragment` (`self.Ref_TPC`)) (`self.CurrentNbFragments`)))
            (set `/Game/CosmicPlatformer/Blueprints/Player/ThirdPersonCharacter.MajorFragment` 0 (`self.Ref_TPC`))
            (goto _label)
            (else
              ;[1 1 1] If False, check if TPC is having more than needed Fragments (should always be True in that case)
              (if (> (`/Game/CosmicPlatformer/Blueprints/Player/ThirdPersonCharacter.MajorFragment` (`self.Ref_TPC`)) (`self.NbFragmentsMissing`))
                ;[1 1 1] Gives to the NPC the required number of Fragments and refreshes TPC's number of Fragments
                (set `/Game/CosmicPlatformer/Blueprints/Player/ThirdPersonCharacter.MajorFragment` (- (`/Game/CosmicPlatformer/Blueprints/Player/ThirdPersonCharacter.MajorFragment` (`self.Ref_TPC`)) (`self.NbFragmentsMissing`)) (`self.Ref_TPC`))
                (set `self.CurrentNbFragments` (`self.NbFragmentsNeeded`))
                (goto _label)))))))
    (:`NewEnumerator1`
      ;[1 1 1] If Minor, just sets the text to display
      (set `self.TexteToFill` (`self.MinorNPC_Dialogue`))
      (goto _label_2))))

(event `Disappear`
  (`KismetSystemLibrary.Delay` 3.0)
  (`WidgetComponent.SetWidget` (`self.Widget_Dialogue`) null))

(fn `UserConstructionScript`
  (`parent.UserConstructionScript`))
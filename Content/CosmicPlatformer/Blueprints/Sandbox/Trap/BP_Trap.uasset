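; Trap actor that swings its Pivot open when the third-person character overlaps its Sphere.
; A DoOnce gates activation, prints a "Clic" debug string, then after a short delay a timeline rotates the Pivot to -90 degrees pitch or yaw.
; A TrapDuration delay, started from that timeline's update, leads to a second timeline that sets the Pivot to zero rotation and re-arms the DoOnce.
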(event `self.Sphere.OnComponentBeginOverlap`
  (params (OverlappedComponent :type "PrimitiveComponent Object Reference") (OtherActor :type "Actor Object Reference") (OtherComp :type "PrimitiveComponent Object Reference") (OtherBodyIndex :type Integer) (bFromSweep :type Boolean) (SweepResult :type "HitResult Structure (by ref)"))
  (cast `/Game/CosmicPlatformer/Blueprints/Player/ThirdPersonCharacter` OtherActor)
  (`self.TrapActivation`))

(event `TrapActivation`
  (`/Engine/EditorBlueprintResources/StandardMacros.DoOnce` false :!label _label
    (:`Completed`
      (`KismetSystemLibrary.PrintString` "Clic")
      (`KismetSystemLibrary.Delay` 0.5)
      (bind (_direction _newtrack_0) (`Timeline|TrapTL1` :!via `PlayFromStart`)
        (:`Update`
          (`SceneComponent.K2_SetRelativeRotation` (`self.Pivot`) (`KismetMathLibrary.RLerp` (struct) (struct :`Pitch` -90.0) _newtrack_0) false false)
          (`KismetSystemLibrary.Delay` (`self.TrapDuration`))
          (bind (_direction_2 _newtrack_0_2) (`Timeline|TrapTL2`)
            (:`Update`
              (`SceneComponent.K2_SetRelativeRotation` (`self.Pivot`) (`KismetMathLibrary.RLerp` (struct) (struct) _newtrack_0_2) false false)
              (goto _label :!via `Reset`))))))))

(fn `UserConstructionScript`)
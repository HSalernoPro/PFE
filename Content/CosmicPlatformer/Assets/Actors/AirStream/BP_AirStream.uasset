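; BP_AirStream is an air current volume that pushes the third-person player character upward while they are inside it.
; Box overlap begin stores the character in RefPlayer and disables its gliding; overlap end re-enables gliding and clears the reference.
; While the reference is valid, Tick adds a fixed upward velocity-change impulse to the character's movement each frame, without scaling by delta time.
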(event `self.ReceiveTick`
  (params (DeltaSeconds :type "Float (single-precision)"))
  (bind _ref_player (`self.Ref_Player`))
  (`/Engine/EditorBlueprintResources/StandardMacros.IsValid` _ref_player
    (:`Is Valid`
      (`CharacterMovementComponent.AddImpulse` (`Character.CharacterMovement` _ref_player) (0.0 0.0 42.0) true))))

(event `self.Box.OnComponentBeginOverlap`
  (params (OverlappedComponent :type "PrimitiveComponent Object Reference") (OtherActor :type "Actor Object Reference") (OtherComp :type "PrimitiveComponent Object Reference") (OtherBodyIndex :type Integer) (bFromSweep :type Boolean) (SweepResult :type "HitResult Structure (by ref)"))
  (bind _asthird_person_character (cast `/Game/CosmicPlatformer/Blueprints/Player/ThirdPersonCharacter` OtherActor))
  (bind _output_get (set `self.Ref_Player` _asthird_person_character))
  (set `/Game/CosmicPlatformer/Blueprints/Player/ThirdPersonCharacter.CanGlide?` false _output_get))

(event `self.Box.OnComponentEndOverlap`
  (params (OverlappedComponent :type "PrimitiveComponent Object Reference") (OtherActor :type "Actor Object Reference") (OtherComp :type "PrimitiveComponent Object Reference") (OtherBodyIndex :type Integer))
  (cast `/Game/CosmicPlatformer/Blueprints/Player/ThirdPersonCharacter` OtherActor)
  (set `/Game/CosmicPlatformer/Blueprints/Player/ThirdPersonCharacter.CanGlide?` true (`self.Ref_Player`))
  (set `self.Ref_Player` null))

(fn `UserConstructionScript`)
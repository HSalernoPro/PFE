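; BP_Trampoline is a trampoline actor that tells ThirdPersonCharacter when a trampoline super jump is available.
; Entering BoxSuperJump with non-zero vertical velocity sets the character's TrampolineJump flag and trampoline reference; leaving it or entering BoxCollision clears the flag.
; SuperJumpTriggered only sets the bounce multipliers.
; The velocity-inverting LaunchCharacter bounce is disconnected, so this Blueprint launches nothing itself.
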(event `self.BoxCollision.OnComponentBeginOverlap`
  (params (OverlappedComponent :type "PrimitiveComponent Object Reference") (OtherActor :type "Actor Object Reference") (OtherComp :type "PrimitiveComponent Object Reference") (OtherBodyIndex :type Integer) (bFromSweep :type Boolean) (SweepResult :type "HitResult Structure (by ref)"))
  (bind _asthird_person_character (cast `/Game/CosmicPlatformer/Blueprints/Player/ThirdPersonCharacter` OtherActor))
  (set `/Game/CosmicPlatformer/Blueprints/Player/ThirdPersonCharacter.TrampolineJump` false _asthird_person_character)
  (if (`self.HasSuperJump?`)
    _))

(event `self.BoxSuperJump.OnComponentBeginOverlap`
  (params (OverlappedComponent :type "PrimitiveComponent Object Reference") (OtherActor :type "Actor Object Reference") (OtherComp :type "PrimitiveComponent Object Reference") (OtherBodyIndex :type Integer) (bFromSweep :type Boolean) (SweepResult :type "HitResult Structure (by ref)"))
  (bind _asthird_person_character (cast `/Game/CosmicPlatformer/Blueprints/Player/ThirdPersonCharacter` OtherActor))
  (if (not (== (.z (`self.GetVelocity` _asthird_person_character)) 0.0))
    (set `/Game/CosmicPlatformer/Blueprints/Player/ThirdPersonCharacter.TrampolineJump` true _asthird_person_character)
    (set `/Game/CosmicPlatformer/Blueprints/Player/ThirdPersonCharacter.Ref_Trampoline` self _asthird_person_character)))

(event `self.BoxSuperJump.OnComponentEndOverlap`
  (params (OverlappedComponent :type "PrimitiveComponent Object Reference") (OtherActor :type "Actor Object Reference") (OtherComp :type "PrimitiveComponent Object Reference") (OtherBodyIndex :type Integer))
  (bind _asthird_person_character (cast `/Game/CosmicPlatformer/Blueprints/Player/ThirdPersonCharacter` OtherActor))
  (set `/Game/CosmicPlatformer/Blueprints/Player/ThirdPersonCharacter.TrampolineJump` false _asthird_person_character))

(event `SuperJumpTriggered`
  (set `self.ConstantJump` -1.0)
  (set `self.JumpStrength` 1.0))

(fn `UserConstructionScript`)
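; Moving platform that travels between its starting relative location and a targeted location, optionally ping-ponging when Loop is set.
; A timeline lerps the cube's position, with PlateformSpeed scaling the play rate and a near-zero speed defaulting to 1.
; It starts on BeginPlay or, with ActivationThxToCollision, plays only while the ThirdPersonCharacter overlaps its box, pausing on exit and resuming on re-entry.
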(event `self.ReceiveBeginPlay`
  (bind _movement_timeline (`self.Movement_Timeline`))
  ;[1 1 1] At the beginning, get the location of the plateform and saves it.
  (set `self.Start_Location` (`SceneComponent.RelativeLocation` (`self.Plateform_Cube`)))
  ;[1 1 1] Check if the person who put the plateform forgotten or not to put a speed, if so, set it to 1.
  (if (`KismetMathLibrary.NearlyEqual_FloatFloat` (`self.PlateformSpeed`) 0.0 0.01)
    (set `self.PlateformSpeed` 1.0))
  ;[1 1 1] Sets the Speed of the plateform.
  (`TimelineComponent.SetPlayRate` _movement_timeline (* (`TimelineComponent.GetTimelineLength` _movement_timeline) (`self.PlateformSpeed`)))
  ;[1 1 1] Check if we want to activate the plateform thanks to the Character or not, if not, then it'll immediatly starts moving.
  (if (not (`self.ActivationThxToCollision?`))
    ;[1 1 1] Float Timeline of 1 second. Values are useless. The only thing that matters is the 1 second of the Timeline.
    ; Causes to lerp from the start location to the targeted location over that time, which can be manipulated by "PlateformSpeed".
    (bind (_direction _movementduration) (`Timeline|Movement_Timeline` :!via `PlayFromStart` :!label _label)
      (:`Update`
        (`SceneComponent.K2_SetRelativeLocation` (`self.Plateform_Cube`) (`KismetMathLibrary.VLerp` (`self.Start_Location`) (`self.Targeted_Location`) _movementduration) false false))
      (:`Finished`
        ;[1 1 1] Whether or not the plateform does round trip.
        (if (`self.Loop?`)
          (`/Engine/EditorBlueprintResources/StandardMacros.FlipFlop`
            (:`A`
              (goto _label :!via `Reverse`))
            (:`B`
              (goto _label))))))))

(event `self.Box_Collision.OnComponentBeginOverlap`
  (params (OverlappedComponent :type "PrimitiveComponent Object Reference") (OtherActor :type "Actor Object Reference") (OtherComp :type "PrimitiveComponent Object Reference") (OtherBodyIndex :type Integer) (bFromSweep :type Boolean) (SweepResult :type "HitResult Structure (by ref)"))
  ;[1 1 1] Starts Timeline upon colliding with the plateform and STOPS the timeline when moving out. Restarts from where it sopped if step again on it.
  (cast `/Game/CosmicPlatformer/Blueprints/Player/ThirdPersonCharacter` OtherActor)
  ;[1 1 1] Check if we want to activate the plateform thanks to the Character or not, if not, then it'll immediatly starts moving.
  (if (`self.ActivationThxToCollision?`)
    (goto _label)))

(event `self.Box_Collision.OnComponentEndOverlap`
  (params (OverlappedComponent :type "PrimitiveComponent Object Reference") (OtherActor :type "Actor Object Reference") (OtherComp :type "PrimitiveComponent Object Reference") (OtherBodyIndex :type Integer))
  ;[1 1 1] Starts Timeline upon colliding with the plateform and STOPS the timeline when moving out. Restarts from where it sopped if step again on it.
  (cast `/Game/CosmicPlatformer/Blueprints/Player/ThirdPersonCharacter` OtherActor)
  ;[1 1 1] Check if we want to activate the plateform thanks to the Character or not, if not, then it'll immediatly starts moving.
  (if (`self.ActivationThxToCollision?`)
    (goto _label :!via `Stop`)))

(fn `UserConstructionScript`)
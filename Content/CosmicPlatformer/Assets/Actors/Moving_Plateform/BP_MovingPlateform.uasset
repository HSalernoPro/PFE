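; Configurable platformer platform that can move, loop back and forth, and break when stepped on.
; A timeline lerps the cube from its start to an arrival marker captured and destroyed at BeginPlay, with speed set through play rate.
; Movement starts automatically, while the character overlaps the box, or through external trigger events.
; Breakable platforms count character overlaps, then hide, drop collision and respawn after a delay, optionally restarting their movement.
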(event `StartThxToTrigger`
  ;[1 1 1] Related to Trigger
  ;[1 1 1] Float Timeline of 1 second. Values are useless. The only thing that matters is the 1 second of the Timeline.
  ; Causes to lerp from the start location to the targeted location over that time, which can be manipulated by "PlateformSpeed".
  (bind (_direction _movementduration) (`Timeline|Movement_Timeline` :!label _label)
    (:`Update`
      (`SceneComponent.K2_SetRelativeLocation` (`self.Plateform_Cube`) (`KismetMathLibrary.VLerp` (`self.StartLocation`) (`self.TargetedLocation`) _movementduration) false false))
    (:`Finished`
      ;[1 1 1] Whether or not the plateform does round trip.
      (if (`self.Loop?`)
        (`/Engine/EditorBlueprintResources/StandardMacros.FlipFlop`
          (:`A`
            (goto _label :!via `Reverse`))
          (:`B`
            (goto _label)))))))

(event `RecallSpeed`
  (bind _movement_timeline (`self.Movement_Timeline`))
  ;[1 1 1] Sets the Speed of the plateform.
  (`TimelineComponent.SetPlayRate` _movement_timeline (* (`TimelineComponent.GetTimelineLength` _movement_timeline) (`self.PlateformSpeed`)) :!label _label_2)
  ;[1 1 1] Check if we want to activate the plateform thanks to the Character or not, if not, then it'll immediatly starts moving.
  (if (not (`self.ActivationThxToCollision?`))
    ;[1 1 1] Related to Trigger
    (if (not (`self.TriggerActivation?`))
      (goto _label :!via `PlayFromStart`))))

(event `StopThxToTrigger`
  ;[1 1 1] Related to Trigger
  (goto _label :!via `Stop`))

(event `self.ReceiveBeginPlay`
  (bind _plateformarrival (`self.PlateformArrival`))
  ;[1 1 1] At the beginning, get the location of the plateform and saves it.
  (set `self.StartLocation` (`SceneComponent.RelativeLocation` (`self.Plateform_Cube`)))
  (set `self.TargetedLocation` (`SceneComponent.K2_GetComponentLocation` _plateformarrival))
  (`ActorComponent.K2_DestroyComponent` _plateformarrival)
  (`PrimitiveComponent.SetMaterial` (`self.Plateform_Cube`) 0 "/Engine/BasicShapes/BasicShapeMaterial.BasicShapeMaterial")
  (if (`self.MovingPlateform?`)
    ;[1 1 1] Check if the person who put the plateform forgotten or not to put a speed, if so, set it to 1.
    (if (== (`self.PlateformSpeed`) 0.0)
      (set `self.PlateformSpeed` 1.0)
      (goto _label_2)
      (else
        (goto _label_2)))))

(event `self.Box_Collision.OnComponentBeginOverlap`
  (params (OverlappedComponent :type "PrimitiveComponent Object Reference") (OtherActor :type "Actor Object Reference") (OtherComp :type "PrimitiveComponent Object Reference") (OtherBodyIndex :type Integer) (bFromSweep :type Boolean) (SweepResult :type "HitResult Structure (by ref)"))
  (bind _plateform_cube (`self.Plateform_Cube`))
  ;[1 1 1] Starts Timeline upon colliding with the plateform and STOPS the timeline when moving out. Restarts from where it sopped if step again on it.
  (cast `/Game/CosmicPlatformer/Blueprints/Player/ThirdPersonCharacter` OtherActor)
  (if (`self.Breakable?`)
    (bind _result (`/Engine/EditorBlueprintResources/StandardMacros.IncrementInt` (`self.NTimesSteppedOnIt`))
      (:`  `
        (if (== _result (`self.NTimesToBreak`))
          (`|ExecutionSequence`
            (:`then_0`
              (goto _label :!via `Stop`))
            (:`then_1`
              (if (`self.ForceRespawnAtStartLocation?`)
                (`self.K2_SetActorLocation` (`self.StartLocation`)))
              (`PrimitiveComponent.SetCollisionEnabled` _plateform_cube "NoCollision")
              (`SceneComponent.SetVisibility` _plateform_cube false false)
              (`self.RespawnEvent`)
              ;[1 1 1] Check if we want to activate the plateform thanks to the Character or not, if not, then it'll immediatly starts moving.
              (if (`self.ActivationThxToCollision?`) :!label _label_3
                (goto _label)))))))
    (else
      (goto _label_3))))

(event `self.Box_Collision.OnComponentEndOverlap`
  (params (OverlappedComponent :type "PrimitiveComponent Object Reference") (OtherActor :type "Actor Object Reference") (OtherComp :type "PrimitiveComponent Object Reference") (OtherBodyIndex :type Integer))
  ;[1 1 1] Starts Timeline upon colliding with the plateform and STOPS the timeline when moving out. Restarts from where it sopped if step again on it.
  (cast `/Game/CosmicPlatformer/Blueprints/Player/ThirdPersonCharacter` OtherActor)
  ;[1 1 1] Check if we want to activate the plateform thanks to the Character or not, if not, then it'll immediatly starts moving.
  (if (`self.ActivationThxToCollision?`)
    (goto _label :!via `Stop`)))

(event `RespawnEvent`
  (bind _plateform_cube (`self.Plateform_Cube`))
  (set `self.NTimesSteppedOnIt` 0)
  (`KismetSystemLibrary.Delay` (`self.RespawnTime`))
  (`PrimitiveComponent.SetCollisionEnabled` _plateform_cube "QueryAndPhysics")
  (`SceneComponent.SetVisibility` _plateform_cube true true)
  (if (`self.WasOn?`)
    (if (`self.ForceRespawnAtStartLocation?`)
      (goto _label :!via `PlayFromStart`)
      (else
        (goto _label)))))

(fn `UserConstructionScript`)
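; BP_TriggerMovingPlat is a trigger that lets the player start and stop a moving platform with the E key.
; On BeginPlay it caches the start and arrival marker positions, destroys the markers, then spawns a BP_MovingPlateform configured with its movement, loop, breakable and respawn settings.
; Box overlap with the ThirdPersonCharacter arms the trigger, and a FlipFlop alternates start and stop calls while updating the platform's WasOn flag.
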(event `self.ReceiveBeginPlay`
  (bind _plateformstart (`self.PlateformStart`))
  (bind _plateformarrival (`self.PlateformArrival`))
  (set `self.StartLocation` (`SceneComponent.K2_GetComponentLocation` _plateformstart))
  (`ActorComponent.K2_DestroyComponent` _plateformstart)
  (set `self.TargetedLocation` (`SceneComponent.K2_GetComponentLocation` _plateformarrival))
  (`ActorComponent.K2_DestroyComponent` _plateformarrival)
  (`self.EnableInput` self (`GameplayStatics.GetPlayerController` 0))
  (bind _returnvalue (`|SpawnActorFromClass` "/Game/CosmicPlatformer/Assets/Actors/Moving_Plateform/BP_MovingPlateform.BP_MovingPlateform_C" (`KismetMathLibrary.MakeTransform` (`self.StartLocation`) (struct) (`self.PlateformScale`)) "Undefined" "OverrideRootScale" null null))
  (bind _output_get (set `self.RefMovingPlateform` _returnvalue))
  (set `/Game/CosmicPlatformer/Assets/Actors/Moving_Plateform/BP_MovingPlateform.TargetedLocation` (`self.TargetedLocation`) _output_get)
  (set `/Game/CosmicPlatformer/Assets/Actors/Moving_Plateform/BP_MovingPlateform.MovingPlateform?` true _output_get)
  (set `/Game/CosmicPlatformer/Assets/Actors/Moving_Plateform/BP_MovingPlateform.Loop?` (`self.Loop?`) _output_get)
  (set `/Game/CosmicPlatformer/Assets/Actors/Moving_Plateform/BP_MovingPlateform.TriggerActivation?` true _output_get)
  (set `/Game/CosmicPlatformer/Assets/Actors/Moving_Plateform/BP_MovingPlateform.PlateformSpeed` (`self.PlateformSpeed`) _output_get)
  (set `/Game/CosmicPlatformer/Assets/Actors/Moving_Plateform/BP_MovingPlateform.Breakable?` (`self.Breakable?`) _output_get)
  (set `/Game/CosmicPlatformer/Assets/Actors/Moving_Plateform/BP_MovingPlateform.NTimesToBreak` (`self.NTimesToBreak`) _output_get)
  (set `/Game/CosmicPlatformer/Assets/Actors/Moving_Plateform/BP_MovingPlateform.RespawnTime` (`self.RespawnTime`) _output_get)
  (set `/Game/CosmicPlatformer/Assets/Actors/Moving_Plateform/BP_MovingPlateform.ForceRespawnAtStartLocation?` (`self.ForceRespawnAtStartLocation?`) _output_get)
  (set `/Game/CosmicPlatformer/Assets/Actors/Moving_Plateform/BP_MovingPlateform.WasOn?` false _output_get))

(event `self.Box.OnComponentBeginOverlap`
  (params (OverlappedComponent :type "PrimitiveComponent Object Reference") (OtherActor :type "Actor Object Reference") (OtherComp :type "PrimitiveComponent Object Reference") (OtherBodyIndex :type Integer) (bFromSweep :type Boolean) (SweepResult :type "HitResult Structure (by ref)"))
  (cast `/Game/CosmicPlatformer/Blueprints/Player/ThirdPersonCharacter` OtherActor)
  (set `self.TriggerAvailable` true))

(event `self.Box.OnComponentEndOverlap`
  (params (OverlappedComponent :type "PrimitiveComponent Object Reference") (OtherActor :type "Actor Object Reference") (OtherComp :type "PrimitiveComponent Object Reference") (OtherBodyIndex :type Integer))
  (cast `/Game/CosmicPlatformer/Blueprints/Player/ThirdPersonCharacter` OtherActor)
  (set `self.TriggerAvailable` false))

(event `Key|E`
  (params (Key :type "Key Structure"))
  (bind _refmovingplateform (`self.RefMovingPlateform`))
  (:`Pressed`
    (if (`self.TriggerAvailable`)
      (`/Engine/EditorBlueprintResources/StandardMacros.FlipFlop`
        (:`A`
          (`/Game/CosmicPlatformer/Assets/Actors/Moving_Plateform/BP_MovingPlateform.StartThxToTrigger` _refmovingplateform)
          (set `/Game/CosmicPlatformer/Assets/Actors/Moving_Plateform/BP_MovingPlateform.WasOn?` true _refmovingplateform))
        (:`B`
          (`/Game/CosmicPlatformer/Assets/Actors/Moving_Plateform/BP_MovingPlateform.StopThxToTrigger` _refmovingplateform)
          (set `/Game/CosmicPlatformer/Assets/Actors/Moving_Plateform/BP_MovingPlateform.WasOn?` false _refmovingplateform))))))

(fn `UserConstructionScript`)
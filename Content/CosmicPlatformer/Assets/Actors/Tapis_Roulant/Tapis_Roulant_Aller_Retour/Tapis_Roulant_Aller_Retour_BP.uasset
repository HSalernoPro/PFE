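; Back-and-forth conveyor belt actor that carries overlapping actors and periodically reverses direction in the platformer.
; Tick offsets every actor in BoxCollisionTapis along the Tapis mesh's forward vector, scaled by Vitesse.
; BeginPlay runs an endless Delay loop cycling forward, paused and reverse phases, setting Vitesse and swapping new dynamic material instances to match.
; Construction script applies configurable arrow color, speed and scale, though the loop later uses hardcoded values.
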(event `self.ReceiveTick`
  (params (DeltaSeconds :type "Float (single-precision)"))
  (for _array_element (`PrimitiveComponent.GetOverlappingActors` (`self.Box_Collision_Tapis`) null)
    (`self.K2_AddActorWorldOffset` _array_element (* (`KismetMathLibrary.GetForwardVector` (`SceneComponent.K2_GetComponentRotation` (`self.Tapis`))) (* DeltaSeconds (`self.Vitesse`))) false false)))

(event `self.ReceiveBeginPlay`
  (bind _tapis (`self.Tapis`))
  (set `self.Vitesse` 125.0)
  (`KismetSystemLibrary.Delay` (`self.Delay_avant_permutation`) :!label _label)
  (bind _returnvalue (`PrimitiveComponent.CreateDynamicMaterialInstance` _tapis 0 "/Game/CosmicPlatformer/Assets/Actors/Tapis_Roulant/Tapis_Roulant_Interruption_M.Tapis_Roulant_Interruption_M" "None"))
  (`PrimitiveComponent.SetMaterial` _tapis 0 _returnvalue)
  (set `self.Vitesse` 0.0)
  (`MeshComponent.SetVectorParameterValueOnMaterials` _tapis "Couleur" (1.0 0.0 0.866667))
  (`KismetSystemLibrary.Delay` (`self.Delay_Interruption`))
  (bind _returnvalue_2 (`PrimitiveComponent.CreateDynamicMaterialInstance` _tapis 0 "/Game/CosmicPlatformer/Assets/Actors/Tapis_Roulant/Tapis_Roulant_Retour_M.Tapis_Roulant_Retour_M" "None"))
  (`PrimitiveComponent.SetMaterial` _tapis 0 _returnvalue_2)
  (`MeshComponent.SetScalarParameterValueOnMaterials` _tapis "Echelle_de_X" -3.0)
  (set `self.Vitesse` -125.0)
  (`MeshComponent.SetScalarParameterValueOnMaterials` _tapis "Vitesse_de_X" -0.45)
  (`MeshComponent.SetVectorParameterValueOnMaterials` _tapis "Couleur" (1.0 0.0 0.866667))
  (`KismetSystemLibrary.Delay` (`self.Delay_avant_permutation`))
  (bind _returnvalue_3 (`PrimitiveComponent.CreateDynamicMaterialInstance` _tapis 0 "/Game/CosmicPlatformer/Assets/Actors/Tapis_Roulant/Tapis_Roulant_Interruption_M.Tapis_Roulant_Interruption_M" "None"))
  (`PrimitiveComponent.SetMaterial` _tapis 0 _returnvalue_3)
  (set `self.Vitesse` 0.0)
  (`MeshComponent.SetVectorParameterValueOnMaterials` _tapis "Couleur" (1.0 0.0 0.866667))
  (`KismetSystemLibrary.Delay` (`self.Delay_Interruption`))
  (bind _returnvalue_4 (`PrimitiveComponent.CreateDynamicMaterialInstance` _tapis 0 "/Game/CosmicPlatformer/Assets/Actors/Tapis_Roulant/Tapis_Roulant_M.Tapis_Roulant_M" "None"))
  (`PrimitiveComponent.SetMaterial` _tapis 0 _returnvalue_4)
  (`MeshComponent.SetScalarParameterValueOnMaterials` _tapis "Echelle_de_X" 3.0)
  (`MeshComponent.SetScalarParameterValueOnMaterials` _tapis "Vitesse_de_X" -0.45)
  (`MeshComponent.SetVectorParameterValueOnMaterials` _tapis "Couleur" (1.0 0.0 0.866667))
  (set `self.Vitesse` 125.0)
  (goto _label))

(fn `UserConstructionScript`
  (bind _tapis (`self.Tapis`))
  (bind _returnvalue (`PrimitiveComponent.CreateDynamicMaterialInstance` _tapis 0 "/Game/CosmicPlatformer/Assets/Actors/Tapis_Roulant/Tapis_Roulant_M.Tapis_Roulant_M" "None"))
  (`PrimitiveComponent.SetMaterial` _tapis 0 _returnvalue)
  ;[1 1 1] Permet de changer la couleur des flèches.
  (`MaterialInstanceDynamic.SetVectorParameterValue` _returnvalue "Couleur" (`self.ValeursCouleur`))
  ;[1 1 1] Vitesse des Flèches
  (`MaterialInstanceDynamic.SetScalarParameterValue` _returnvalue "Vitesse_de_X" (`self.Vitesse_Fleches`))
  ;[1 1 1] Variable pour modifier le nombre et la direction des flèches.
  (`MaterialInstanceDynamic.SetScalarParameterValue` _returnvalue "Echelle_de_X" (`self.Echelle_Fleches`)))
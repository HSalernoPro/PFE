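; Conveyor belt actor that pushes any actor standing on it along the belt.
; Each tick, every actor overlapping the belt's collision box is offset along the belt mesh's forward vector by speed times delta time, without sweep.
; The construction script gives the mesh a dynamic material instance, setting arrow color, scale and scroll speed from variables separate from the push speed.
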(event `self.ReceiveTick`
  (params (DeltaSeconds :type "Float (single-precision)"))
  (for _array_element (`PrimitiveComponent.GetOverlappingActors` (`self.Box_Collision_Tapis`) null)
    (`self.K2_AddActorWorldOffset` _array_element (* (`KismetMathLibrary.GetForwardVector` (`SceneComponent.K2_GetComponentRotation` (`self.Tapis`))) (* DeltaSeconds (`self.Vitesse`))) false false)))

(fn `UserConstructionScript`
  (bind _tapis (`self.Tapis`))
  (bind _returnvalue (`PrimitiveComponent.CreateDynamicMaterialInstance` _tapis 0 "/Game/CosmicPlatformer/Assets/Actors/Tapis_Roulant/Tapis_Roulant_M.Tapis_Roulant_M" "None"))
  (`PrimitiveComponent.SetMaterial` _tapis 0 _returnvalue)
  ;[1 1 1] Permet de changer la couleur des flèches.
  (`MaterialInstanceDynamic.SetVectorParameterValue` _returnvalue "Couleur" (`self.ValeursCouleur`))
  ;[1 1 1] Reminder pour moi-même : Valeur à toucher pour changer la direction des flèches et leur nombre.
  (`MaterialInstanceDynamic.SetScalarParameterValue` _returnvalue "Echelle_de_X" (`self.Echelle_Fleches`))
  ;[1 1 1] Vitesse du Tapis Roulant
  (`MaterialInstanceDynamic.SetScalarParameterValue` _returnvalue "Vitesse_de_X" (`self.Vitesse_Fleches`)))
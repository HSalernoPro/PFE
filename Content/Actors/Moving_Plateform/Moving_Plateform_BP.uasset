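; Moving platform actor that slides its cube from its starting relative position to a target location.
; A timeline lerps the position, with a FlipFlop alternating reverse and play when looping is enabled.
; BeginPlay applies the scale and either auto-starts the timeline at a speed-derived play rate or leaves it to collision.
; In collision mode, the third-person character entering the box plays the timeline and leaving it stops it.
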(event `self.ReceiveBeginPlay`
  (bind _movement_timeline (`self.Movement_Timeline`))
  (`self.SetActorScale3D` (`self.PlateformScale`))
  (set `self.Start_Location` (`SceneComponent.RelativeLocation` (`self.Plateform_Cube`)))
  (if (`KismetMathLibrary.NearlyEqual_FloatFloat` (`self.PlateformSpeed`) 0.0 0.01)
    (set `self.PlateformSpeed` 1.0))
  (if (not (`self.ActivationThxToCollision?`))
    (`TimelineComponent.SetPlayRate` _movement_timeline (* (`TimelineComponent.GetTimelineLength` _movement_timeline) (`self.PlateformSpeed`)))
    (bind (_direction _movementduration) (`Timeline|Movement_Timeline` :!via `PlayFromStart` :!label _label)
      (:`Update`
        (`SceneComponent.K2_SetRelativeLocation` (`self.Plateform_Cube`) (`KismetMathLibrary.VLerp` (`self.Start_Location`) (`self.Targeted_Location`) _movementduration) false false))
      (:`Finished`
        (if (`self.Loop?`)
          (`/Engine/EditorBlueprintResources/StandardMacros.FlipFlop`
            (:`A`
              (goto _label :!via `Reverse`))
            (:`B`
              (goto _label))))))))

(event `self.Box_Collision.OnComponentBeginOverlap`
  (params (OverlappedComponent :type "PrimitiveComponent Object Reference") (OtherActor :type "Actor Object Reference") (OtherComp :type "PrimitiveComponent Object Reference") (OtherBodyIndex :type Integer) (bFromSweep :type Boolean) (SweepResult :type "HitResult Structure (by ref)"))
  (cast `/Game/CosmicPlatformer/Blueprints/Player/ThirdPersonCharacter` OtherActor)
  (if (`self.ActivationThxToCollision?`)
    (goto _label)))

(event `self.Box_Collision.OnComponentEndOverlap`
  (params (OverlappedComponent :type "PrimitiveComponent Object Reference") (OtherActor :type "Actor Object Reference") (OtherComp :type "PrimitiveComponent Object Reference") (OtherBodyIndex :type Integer))
  (cast `/Game/CosmicPlatformer/Blueprints/Player/ThirdPersonCharacter` OtherActor)
  (if (`self.ActivationThxToCollision?`)
    (goto _label :!via `Stop`)))

(fn `UserConstructionScript`)